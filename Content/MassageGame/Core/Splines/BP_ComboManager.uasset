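; BP_ComboManager runs one combo in the massage game, a group of strokes switched on and off together.
; CheckSuccess fires BP_StrokeManager's success event when Counter matches the stroke count, then clears the player's CurrentCombo.
; While active, it answers that event by enabling NextCombo or, failing that, swapping the current combo's strokes for NextStroke.
; A looping timer decrements Counter between strokes.
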(event Custom|Countdown
  ;[0.3065 1 0.2281 0.309] Supposed to call the function every N seconds
  (bind _returnvalue (Utilities|Time|SetTimerbyFunctionName 0 "DecreaseCounter" (Variables|Default|GetDelayBetwStrokes) true))
  (Variables|Default|SetTimer _returnvalue))

(event Custom|ComboSuccessful
  (bind _returnvalue (Game|Player|GetPlayerPawn 0))
  (bind _asbp_player_character (Utilities|Casting|CastToBP_PlayerCharacter _returnvalue))
  (bind _currentcombo (Variables|/Game/MassageGame/Core/GameMode/BP_PlayerCharacter.BP_PlayerCharacter_C|GetCurrentCombo _asbp_player_character))
  (bind _combostrokes (Variables|BP_ComboManager_C|GetComboStrokes _currentcombo))
  (if (Variables|Default|GetIsActive)
    ;[0.3065 1 0.2281 0.309] basically it's a branch if the next thing is a combo or a single stroke
    (Utilities|IsValid (Variables|Default|GetNextCombo)
      (:Is%20Valid
        (CallFunction|TurnComboOn/Off (Variables|Default|GetNextCombo) true)
        (CallFunction|TurnComboOn/Off (Variables|/Game/MassageGame/Core/GameMode/BP_PlayerCharacter.BP_PlayerCharacter_C|GetCurrentCombo (.AsBP%20Player%20Character (Utilities|Casting|CastToBP_PlayerCharacter (Game|Player|GetPlayerPawn 0)))) false))
      (:Is%20Not%20Valid
        ;[1 0.3665 0 0.2] SO the validation helped, cuz I figured out that the error happens because the success even fires in a freshly activated dispatcher (for some reason, which is unknown) -INVESTIGATE why combo manager is activated before the success dispatcher is fired
        (Utilities|IsValid _currentcombo
          (:Is%20Valid
            (Development|PrintString (Utilities|GetDisplayName (Utilities|Array|Get(acopy) _combostrokes)) true true "(R=1.000000,G=0.000000,B=0.091436,A=1.000000)")
            (for _array_element _combostrokes
              (Default|TurnOn/Off _array_element false))
            (for _array_element_2 (Variables|BP_ComboManager_C|GetNextStroke _currentcombo)
              (Default|TurnOn/Off _array_element_2 true))))))))

(event EventBeginPlay
  (bind _returnvalue (Actor|GetActorOfClass "/Game/MassageGame/Core/Splines/BP_StrokeManager.BP_StrokeManager_C"))
  (EventDispatchers|BindEventtoStrokeSuccessful _returnvalue (delegate Custom|ComboSuccessful))
  (if (Variables|Default|GetIsActive)
    (for _array_element (Variables|Default|GetComboStrokes)
      (Default|TurnOn/Off _array_element true))))

(fn ConstructionScript)

(fn CheckSuccess
  (if (== (Variables|Default|GetCounter) (Utilities|Array|Length (Variables|Default|GetComboStrokes)))
    (bind _returnvalue (Actor|GetActorOfClass "/Game/MassageGame/Core/Splines/BP_StrokeManager.BP_StrokeManager_C"))
    (Default|CallStrokeSuccessful _returnvalue)
    (Variables|/Game/MassageGame/Core/GameMode/BP_PlayerCharacter.BP_PlayerCharacter_C|SetCurrentCombo (.AsBP%20Player%20Character (Utilities|Casting|CastToBP_PlayerCharacter (Game|Player|GetPlayerPawn 0))) 0)
    (Variables|Default|SetIsActive false)))

(fn DecreaseCounter
  (if (> (Variables|Default|GetCounter) 0)
    (Math|Integer|DecrementInt (Variables|Default|GetCounter))
    (else
      (Utilities|Time|InvalidateTimerHandle (Variables|Default|GetTimer)))))

(fn TurnComboOn/Off
  (params (TurnOn? :type Boolean))
  (for _array_element (Variables|Default|GetComboStrokes)
    (Default|TurnOn/Off _array_element TurnOn?)
    (Variables|Default|SetIsActive TurnOn?)))