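; BP_Stroke is a spline-defined touch gesture in the massage game, traced through numbered spheres in order.
; Construction places a tagged collision sphere and label at each spline point.
; Each touch restarts a timeout; timeout or a wrong point calls EndStroke, which succeeds if all points were collected.
; Success advances its ComboManager or fires BP_StrokeManager's dispatcher, whose OnSuccess handler enables the next combo or strokes and disables the current stroke.
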(event Custom|TurnOn/Off
  (params (TurnOn? :type Boolean))
  ;[1 0.7196 0] activating the next strokes: turning on the collision and visibility. Same problem with instances here.
  (if TurnOn?
    (for _array_element (Variables|Default|GetCollisionSpheres)
      (Collision|SetCollisionEnabled _array_element "QueryAndPhysics")
      (Development|SetHiddeninGame _array_element false false))
    (else
      (for _array_element_2 (Variables|Default|GetCollisionSpheres)
        (Collision|SetCollisionEnabled _array_element_2 "NoCollision")
        (Development|SetHiddeninGame _array_element_2 true false))))
  (Variables|Default|SetIsActive true))

(event Custom|OnSuccess
  ;[1 0.7196 0] when StrokeSucessful dispatcher is called from StrokeManager, fire this event. MAKE SURE thta this event fires in each instance of the stroke separately, cuz rn I feel like the turning off stroke fires the same logic as the turning on stroke.
  ;;[1 0.3665 0 0.2] same CRUTCH as inside the combo manager - this event for some reason fires straight after the stroke has been activated
  (if (== (Variables|/Game/MassageGame/Core/GameMode/BP_PlayerCharacter.BP_PlayerCharacter_C|GetCurrentStroke (.AsBP%20Player%20Character (Utilities|Casting|CastToBP_PlayerCharacter (Game|Player|GetPlayerPawn 0)))) self)
    (Utilities|IsValid (Variables|Default|GetNextCombo)
      (:Is%20Valid
        (Default|TurnComboOn/Off (Variables|Default|GetNextCombo) true))
      (:Is%20Not%20Valid
        (for _array_element (Variables|Default|GetNextStrokes)
          (CallFunction|TurnOn/Off _array_element true))))
    (CallFunction|TurnOn/Off (Variables|/Game/MassageGame/Core/GameMode/BP_PlayerCharacter.BP_PlayerCharacter_C|GetCurrentStroke (.AsBP%20Player%20Character (Utilities|Casting|CastToBP_PlayerCharacter (Game|Player|GetPlayerPawn 0)))) false)))

(event Custom|EndStroke
  (bind _combomanager (Variables|Default|GetComboManager))
  (CallFunction|StopCountdown)
  ;[1 0.3665 0 0.2] just in case. investigate influence of overvalidation on performance
  (Utilities|IsValid (Variables|Default|GetPlayer%20Character)
    (:Is%20Valid
      _)
    (:Is%20Not%20Valid
      (bind _asbp_player_character (Utilities|Casting|CastToBP_PlayerCharacter (Game|Player|GetPlayerPawn 0)))
      (Variables|Default|SetPlayer%20Character _asbp_player_character)))
  (Utilities|IsValid (Variables|/Game/MassageGame/Core/GameMode/BP_PlayerCharacter.BP_PlayerCharacter_C|GetCurrentStroke (Variables|Default|GetPlayer%20Character))
    (:Is%20Valid
      (if (== (Spline|GetNumberOfSplinePoints (Variables|BP_Stroke_C|GetSpline (Variables|/Game/MassageGame/Core/GameMode/BP_PlayerCharacter.BP_PlayerCharacter_C|GetCurrentStroke (Variables|Default|GetPlayer%20Character)))) (Utilities|Array|Length (Variables|BP_Stroke_C|GetCurrentStrokePoints (Variables|/Game/MassageGame/Core/GameMode/BP_PlayerCharacter.BP_PlayerCharacter_C|GetCurrentStroke (Variables|Default|GetPlayer%20Character)))))
        (Development|PrintString "Success")
        (Utilities|IsValid (Variables|Default|GetComboManager)
          (:Is%20Valid
            ;[0.3065 1 0.2281 0.309] if the current stroke is the part of the combo, ending the stroke sucessfully calls a function in the combo manager to see if the combo is complete
            (Math|Integer|IncrementInt (Variables|/Game/MassageGame/Core/Splines/BP_ComboManager.BP_ComboManager_C|GetCounter _combomanager)
              (:%20%20
                (Default|CheckSuccess _combomanager))))
          (:Is%20Not%20Valid
            ;[1 0.7196 0 0.2] if the stroke is not a part of combo, it calls a dispatcher in the stroke manager. here might be the problem. CHECK how many events does the dispatcher call. Perhaps add checks of activity in the combos and the strokes which are listening to the dispatcher
            (Default|CallStrokeSuccessful (Variables|Default|GetManager))))
        (else
          (Development|PrintString "Failure")))
      (Utilities|Array|Clear (Variables|BP_Stroke_C|GetCurrentStrokePoints (Variables|/Game/MassageGame/Core/GameMode/BP_PlayerCharacter.BP_PlayerCharacter_C|GetCurrentStroke (Variables|Default|GetPlayer%20Character))))
      (Variables|/Game/MassageGame/Core/GameMode/BP_PlayerCharacter.BP_PlayerCharacter_C|SetCurrentStroke (Variables|Default|GetPlayer%20Character) 0))
    (:Is%20Not%20Valid
      (Development|PrintString "StrokeNotValid"))))

(event EventBeginPlay
  ;[0.3065 1 0.2281 0.309] on start - if stroke shouldn't be active from the start, disable collision
  (if (Variables|Default|GetIsActive)
    ;[1 0.1186 0.8812 0.2] Comment
    (for _array_element (Variables|Default|GetCollisionSpheres)
      (Development|SetHiddeninGame _array_element false false)
      ;[0.3065 1 0.2281 0.309] bind an event to it (event will fire on the success)
      (EventDispatchers|BindEventtoStrokeSuccessful (Variables|Default|GetManager) (EventDispatchers|CreateEvent :!event Custom|OnSuccess)))
    (else
      (for _array_element_2 (Variables|Default|GetCollisionSpheres)
        (Collision|SetCollisionEnabled _array_element_2 "NoCollision")
        ;[0.3065 1 0.2281 0.309] set stroke manager (so i don't have to do it manually; there's only one of them anyway)
        (bind _returnvalue (Actor|GetActorOfClass "/Game/MassageGame/Core/Splines/BP_StrokeManager.BP_StrokeManager_C"))
        (Variables|Default|SetManager _returnvalue)
        (EventDispatchers|BindEventtoStrokeSuccessful (Variables|Default|GetManager) (EventDispatchers|CreateEvent :!event Custom|OnSuccess))))))

(event EventActorOnInputTouchEnter
  (params (FingerIndex :type ETouchIndex%20Enum :default "Touch1"))
  (if (Variables|Default|GetIsActive)
    ;[0 0.3099 1 0.2] Comment
    (CallFunction|StartCountdown)
    ;[1 0.7196 0 0.2] is overvalidating harmful to performance?
    (Utilities|IsValid (Variables|Default|GetPlayer%20Character)
      (:Is%20Valid
        _)
      (:Is%20Not%20Valid
        ;[0.3065 1 0.2281 0.309] in case it's the first sphere of the stroke to be overlapped
        (bind _asbp_player_character (Utilities|Casting|CastToBP_PlayerCharacter (Game|Player|GetPlayerPawn 0)))
        (Variables|Default|SetPlayer%20Character _asbp_player_character)))
    (bind _currentstroke (Variables|/Game/MassageGame/Core/GameMode/BP_PlayerCharacter.BP_PlayerCharacter_C|GetCurrentStroke (Variables|Default|GetPlayer%20Character))
      (:then
        (if (== _currentstroke self)
          ;[1 0.3665 0 0.2] shouldn't this be in the beginning? should this even BE here, as technically you can't overlap the sphere if you're not touching the screen
          (if (Variables|/Game/MassageGame/Core/GameMode/BP_PlayerCharacter.BP_PlayerCharacter_C|GetIs%20Held%20Down (Variables|Default|GetPlayer%20Character)) :!label _label
            ;[0.3065 1 0.2281 0.309] check functions' descriptions
            (bind _spherenum (Default|CheckOverlappedSphere (Variables|Default|GetPlayer%20Character)))
            (bind _success_ (CallFunction|AddPointtoCurrentStroke _spherenum))
            ;[0.3065 1 0.2281 0.309] if the wrong point was overlapped, end stroke abruptly
            (if (not _success_)
              (CallFunction|EndStroke :!label _label_2)))
          (else
            (goto _label_2))))
      (:else
        ;[0.3065 1 0.2281 0.309] if stroke belongs to a combo, the combo is saved in the player character
        (bind _output_get (Variables|/Game/MassageGame/Core/GameMode/BP_PlayerCharacter.BP_PlayerCharacter_C|SetCurrentStroke (Variables|Default|GetPlayer%20Character) self))
        (bind _combomanager (Variables|BP_Stroke_C|GetComboManager _output_get)
          (:then
            (bind _output_get_2 (Variables|/Game/MassageGame/Core/GameMode/BP_PlayerCharacter.BP_PlayerCharacter_C|SetCurrentCombo (Variables|Default|GetPlayer%20Character) _combomanager))
            (Development|PrintString (Utilities|GetDisplayName _output_get_2))
            (goto _label))
          (:else
            (goto _label)))))))

(fn ConstructionScript
  (Utilities|Array|Clear (Variables|Default|GetCollisionSpheres))
  (for _index (range 0 (- (Spline|GetNumberOfSplinePoints (Variables|Default|GetSpline)) 1))
    (bind _returnvalue (AddComponent|AddSphereComponent false))
    (bind _returnvalue_2 (Utilities|Array|Add (Variables|Default|GetCollisionSpheres) _returnvalue))
    (Utilities|Array|Add (Variables|/Script/Engine.ActorComponent|GetComponentTags _returnvalue) (Utilities|String|StringToName (Utilities|String|ToString(Integer) _returnvalue_2))))
  (for (_array_element _array_index) (Variables|Default|GetCollisionSpheres)
    (Transformation|SetRelativeLocation _array_element (.location (Spline|GetTransformatSplinePoint (Variables|Default|GetSpline) _array_index "Local" false)) false false)
    (bind _returnvalue_3 (AddComponent|AddTextRenderComponent false (Math|Transform|MakeTransform (.location (Spline|GetTransformatSplinePoint (Variables|Default|GetSpline) _array_index "Local" false)) "90.000000,0.000000,0.000000" "1.000000,1.000000,1.000000")))
    (Rendering|Components|TextRender|SetText _returnvalue_3 (Utilities|Text|ToText(Name) (Utilities|Array|Get(acopy) (Variables|/Script/Engine.ActorComponent|GetComponentTags _array_element))))))

(fn AddPointtoCurrentStroke
  (params (CurrentPointIndex :type Name))
  (bind _currentstrokepoints (Variables|Default|GetCurrentStrokePoints))
  ;[0.3065 1 0.2281 0.309] number tag of the point this event is fired from
  (Variables|Default|SetCurPointIndex (Math|Conversions|ToInteger(Byte) (Utilities|String|ToString(Name) CurrentPointIndex)))
  (if (> (Utilities|Array|Length (Variables|Default|GetCurrentStrokePoints)) 0)
    (if (== (Utilities|Array|Get(acopy) _currentstrokepoints (- (Utilities|Array|Length _currentstrokepoints) 1)) (- (Variables|Default|GetCurPointIndex) 1))
      ;[0.3065 1 0.2281 0.309] add current point to the array
      (Utilities|Array|Add (Variables|Default|GetCurrentStrokePoints) (Variables|Default|GetCurPointIndex))
      (return true)
      (else
        (return false)))
    (else
      ;[0.3065 1 0.2281 0.309] if the current point has index 0, add it to the array, otherwise fail
      (if (== (Variables|Default|GetCurPointIndex) 0)
        (Utilities|Array|Add (Variables|Default|GetCurrentStrokePoints) 0)
        (return true)
        (else
          (return false))))))

(fn StartCountdown
  (bind _returnvalue (Utilities|Time|SetTimerbyFunctionName 0 "EndStroke" (Variables|Default|GetSpeedTimer)))
  (Variables|Default|SetSpeedTimeHandle _returnvalue))

(fn StopCountdown
  (bind _speedtimehandle (Variables|Default|GetSpeedTimeHandle))
  (if (Utilities|Time|IsValidTimerHandle (Variables|Default|GetSpeedTimeHandle))
    (Utilities|Time|PauseTimerbyHandle _speedtimehandle)
    (Utilities|Time|ClearandInvalidateTimerbyHandle _speedtimehandle)
    (else
      (Development|PrintString "Countdown not valid"))))