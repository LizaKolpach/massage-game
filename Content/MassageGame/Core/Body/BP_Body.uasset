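; BP_Body is the body in the massage game, with dynamic materials for its base and contours created at BeginPlay.
; StrokeSuccessful and debug keys 1–3, which also set a target state, call SwitchState, which is currently empty.
; A disconnected chain would update the current state, read its colours from DT_BodyStates and blend both materials' Color toward them on a Timeline.
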(event Custom|SwitchState)

(event EventStrokeSuccessful
  (CallFunction|SwitchState))

(event EventBeginPlay
  (bind _returnvalue (Rendering|Material|CreateDynamicMaterialInstance (Variables|Default|GetBase) 0 "/Game/MassageGame/Art/Body/MI_Body_Base.MI_Body_Base" "None" :!class /Script/Engine.PrimitiveComponent))
  (Variables|Default|SetBodyMaterial _returnvalue)
  (bind _returnvalue_2 (Rendering|Material|CreateDynamicMaterialInstance (Variables|Default|GetContours) 0 "/Game/MassageGame/Art/Body/MI_Body_Contours.MI_Body_Contours" "None" :!class /Script/Engine.PrimitiveComponent))
  (Variables|Default|SetContourMaterial _returnvalue_2))

(event Input|KeyboardEvents|2
  (params (Key :type Key%20Structure :default "None"))
  ;[1 1 1] debig input
  (:Pressed
    (Variables|Default|SetTargetState "NewEnumerator1")
    (CallFunction|SwitchState)))

(event Input|KeyboardEvents|3
  (params (Key :type Key%20Structure :default "None"))
  ;[1 1 1] debig input
  (:Pressed
    (Variables|Default|SetTargetState "NewEnumerator2")
    (CallFunction|SwitchState)))

(event Input|KeyboardEvents|1
  (params (Key :type Key%20Structure :default "None"))
  ;[1 1 1] debig input
  (:Pressed
    (Variables|Default|SetTargetState "NewEnumerator0")
    (CallFunction|SwitchState)))

(fn ConstructionScript)