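; Player character for the massage game that handles tap-and-drag input and judges strokes on BP_Stroke actors.
; BeginPlay adds the massage Enhanced Input context, and IA_Tap tracks whether the press is held.
; On release, EndStroke compares collected points against the stroke's spline point count, prints success or failure, then resets it.
; CheckOverlappedSphere traces under the cursor, returning a stroke sphere's first tag as its number, plus its owning stroke.
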(event Custom|EndStroke
  (Utilities|IsValid (Variables|Default|GetCurrentStroke)
    (:Is%20Valid
      (if (== (Spline|GetNumberOfSplinePoints (Variables|/Game/MassageGame/Core/Splines/BP_Stroke.BP_Stroke_C|GetSpline (Variables|Default|GetCurrentStroke))) (Utilities|Array|Length (Variables|/Game/MassageGame/Core/Splines/BP_Stroke.BP_Stroke_C|GetCurrentStrokePoints (Variables|Default|GetCurrentStroke))))
        (Development|PrintString "Success")
        (else
          (Development|PrintString "Failure")))
      (Utilities|Array|Clear (Variables|/Game/MassageGame/Core/Splines/BP_Stroke.BP_Stroke_C|GetCurrentStrokePoints (Variables|Default|GetCurrentStroke)))
      (Variables|Default|SetCurrentStroke 0))
    (:Is%20Not%20Valid
      (Development|PrintString "StrokeNotValid"))))

(event Input|EnhancedActionEvents|EnhancedInputActionIA_Tap
  (params (ActionValue :type Boolean) (ElapsedSeconds :type Float%20%28double-precision%29) (TriggeredSeconds :type Float%20%28double-precision%29) (InputAction :type Input%20Action%20Object%20Reference :default "/Game/MassageGame/Core/GameMode/IA_Tap.IA_Tap"))
  (:Triggered
    (Variables|Default|SetIs%20Held%20Down true))
  (:Completed
    (Variables|Default|SetIs%20Held%20Down false)
    (CallFunction|EndStroke)))

(event Collision|EventActorBeginOverlap
  (params (OtherActor :type Actor%20Object%20Reference)))

(event EventBeginPlay
  (bind _asbp_player_controller (Utilities|Casting|CastToBP_PlayerController (Game|GetPlayerController 0)))
  (Input|AddMappingContext (PlayerController|LocalPlayerSubsystems|GetEnhancedInputLocalPlayerSubsystem _asbp_player_controller) "/Game/MassageGame/Core/GameMode/IMC_Massage.IMC_Massage" 0 "(bIgnoreAllPressedKeysUntilRelease=True,bForceImmediately=False)"))

(fn ConstructionScript)

(fn CheckOverlappedSphere
  (bind _asbp_player_controller (Utilities|Casting|CastToBP_PlayerController (Game|GetPlayerController 0)))
  (Utilities|Casting|CastToBP_Stroke (.hitactor (.HitResult (Class|PlayerController|GetHitResultUnderCursorforObjects _asbp_player_controller (Variables|Default|GetObject%20Types) true))))
  (bind _assphere_collision (Utilities|Casting|CastToSphereComponent (.hitcomponent (.HitResult (Class|PlayerController|GetHitResultUnderCursorforObjects _asbp_player_controller (Variables|Default|GetObject%20Types) true)))))
  (return (Utilities|Array|Get(acopy) (Variables|/Script/Engine.ActorComponent|GetComponentTags _assphere_collision)) (.AsBP%20Stroke (Utilities|Casting|CastToBP_Stroke (Components|GetOwner _assphere_collision)))))